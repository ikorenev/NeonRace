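; Base car Blueprint that handles driving input, engine audio and rear lights.
; BeginPlay starts the engine and a looping timer that feeds RPM to the SoundEngine, while gear changes swap its sound cue for reverse and six forward gears.
; Input drives throttle/brake, steering and handbrake; throttle axis values of -1 or above also play a timeline ramping rear light intensity.
; Bound race and unrace dispatchers toggle a Race flag.
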(event Custom|Timer
  (Audio|Parameter|SetFloatParameter (Variables|Default|GetSoundEngine) "RPM" (Variables|Default|GetRPM) :!class /Script/AudioExtensions.AudioParameterControllerInterface))

(event Custom|CustomEvent
  (Variables|Default|Setrace true))

(event Custom|CustomEvent_0
  (Variables|Default|Setrace false))

(event EventBeginPlay
  (|CallParentFunction)
  (CallFunction|StartEngine)
  (CallFunction|SetShifterPosition "NewEnumerator3")
  (Components|Activation|Activate (Variables|Default|GetSoundEngine) false)
  (Utilities|Time|SetTimerbyEvent (delegate Custom|Timer) 0.05 true)
  (EventDispatchers|BindEventtoRaceDisp (delegate Custom|CustomEvent))
  (EventDispatchers|BindEventtoUnraceDisp (delegate Custom|CustomEvent_0)))

(event Collision|EventActorBeginOverlap
  (params (OtherActor :type Actor%20Object%20Reference)))

(event EventTick
  (params (DeltaSeconds :type Float%20%28single-precision%29)))

(event EventGearChanged
  (params (PreviousGear :type Integer) (CurrentGear :type Integer))
  (bind _soundengine (Variables|Default|GetSoundEngine))
  ;[1 1 1] Переключение звуков при смене передач
  (switch int CurrentGear
    (:0
      ;;[1 0.2078 0.0478] RearGear
      (Audio|Components|Audio|SetSound _soundengine (Variables|Default|GetRearGearSoundCue)))
    (:1
      ;;[0.2541 0.5536 1] 1stGear
      (Audio|Components|Audio|SetSound _soundengine (Variables|Default|Get1stGearSoundCue)))
    (:2
      ;;[0.2541 0.5536 1] 2ndGear
      (Audio|Components|Audio|SetSound _soundengine (Variables|Default|Get2ndGearSoundCue)))
    (:3
      ;;[0.2541 0.5536 1] 3rdGear
      (Audio|Components|Audio|SetSound _soundengine (Variables|Default|Get3rdGearSoundCue)))
    (:4
      ;;[0.2541 0.5536 1] 4thGear
      (Audio|Components|Audio|SetSound _soundengine (Variables|Default|Get4thGearSoundCue)))
    (:5
      ;;[0.2541 0.5536 1] 5thGear
      (Audio|Components|Audio|SetSound _soundengine (Variables|Default|Get5thGearSoundCue)))
    (:6
      ;;[1 0.2794 0.3291] 6thGear
      (Audio|Components|Audio|SetSound _soundengine (Variables|Default|Get6thGearSoundCue))))
  (Audio|Components|Audio|Play _soundengine 0.0))

(event Input|ActionEvents|InputActionHandbrake
  (params (Key :type Key%20Structure :default "None"))
  (:Pressed
    (CallFunction|SetHandbrakeInput true))
  (:Released
    (CallFunction|SetHandbrakeInput false)))

(event Input|AxisEvents|InputAxisVechicleSteering
  (params (AxisValue :type Float%20%28single-precision%29))
  (CallFunction|SetSteeringInput AxisValue))

(event Input|AxisEvents|InputAxisVehicleThrottle
  (params (AxisValue :type Float%20%28single-precision%29))
  (Math|Float|CompareFloat AxisValue -1.0
    (:>
      (Utilities|FlowControl|Sequence :!label _label
        (:then_0
          (CallFunction|SetThrottleandBrakeInput AxisValue :!label _label_2))
        (:then_1
          (bind _newtrack_0 (Timeline|Light Play)
            (:Update
              (Rendering|Components|Light|SetIntensity (Variables|Default|GetRBackLight) (Math|Float|Lerp 0.0 2e+02 _newtrack_0))
              (Rendering|Components|Light|SetIntensity (Variables|Default|GetLBackLight) (Math|Float|Lerp 0.0 2e+02 _newtrack_0)))))))
    (:==
      (goto _label))
    (:<
      (goto _label_2))))

(fn ConstructionScript
  (|CallParentFunction))
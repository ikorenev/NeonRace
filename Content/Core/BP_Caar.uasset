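; BP_Caar is a player-input-driven car Blueprint built on inherited vehicle functions.
; On BeginPlay it starts the engine and sets the shifter position.
; Throttle and steering axes feed straight into the vehicle inputs, with one axis covering both throttle and brake, while the Handbrake action toggles the handbrake on press and release.
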(event EventBeginPlay
  (|CallParentFunction)
  (CallFunction|StartEngine)
  (CallFunction|SetShifterPosition "NewEnumerator3"))

(event Collision|EventActorBeginOverlap
  (params (OtherActor :type Actor%20Object%20Reference)))

(event EventTick
  (params (DeltaSeconds :type Float%20%28single-precision%29)))

(event Input|ActionEvents|InputActionHandbrake
  (params (Key :type Key%20Structure :default "None"))
  (:Pressed
    (CallFunction|SetHandbrakeInput true))
  (:Released
    (CallFunction|SetHandbrakeInput false)))

(event Input|AxisEvents|InputAxisVechicleSteering
  (params (AxisValue :type Float%20%28single-precision%29))
  (CallFunction|SetSteeringInput AxisValue))

(event Input|AxisEvents|InputAxisVehicleThrottle
  (params (AxisValue :type Float%20%28single-precision%29))
  (CallFunction|SetThrottleandBrakeInput AxisValue))

(fn ConstructionScript
  (|CallParentFunction))
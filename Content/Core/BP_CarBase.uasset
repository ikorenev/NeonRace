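; BP_CarBase is a mostly inactive Blueprint holding logic for a speed-driven post-process effect on the player's car.
; SetPostProcess casts the player pawn to BP_BaseCar, maps rounded air speed to its PostProcess blend weight via an unusually wide Lerp, and prints the ratio.
; The looping timer meant to drive it and the VehicleSetup_HUD creation are disconnected, and BeginPlay is empty, so nothing here triggers the effect.
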(event Custom|Set%20PostProcess
  (bind _asbp_base_car (Utilities|Casting|CastToBP_BaseCar (Game|Player|GetPlayerPawn 0)))
  (Variables|/Script/Engine.PostProcessComponent|SetBlendWeight (Variables|/Game/Core/Cars/BP_BaseCar.BP_BaseCar_C|GetPostProcess _asbp_base_car) (Math|Float|Lerp 0.0 1e+02 (/ (Math|Conversions|ToFloat(Integer) (Class|KismetMathLibrary|Round64 (Default|GetAirSpeed _asbp_base_car))) 1e+02)))
  (Development|PrintString (Utilities|String|ToString(Float) (/ (Math|Conversions|ToFloat(Integer) (Class|KismetMathLibrary|Round64 (Default|GetAirSpeed _asbp_base_car))) 1e+02))))

(event EventBeginPlay)

(event EventTick
  (params (DeltaSeconds :type Float%20%28single-precision%29)))

(fn ConstructionScript)
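; BP_Light_Fonar is a lamp Blueprint with a selectable light color.
; Its construction script switches on the LightColor enum and sets the Light component to a matching purple, red, blue or green color.
; The event graph holds only disabled default events, so the Blueprint adds no runtime logic.
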(event EventBeginPlay)

(event Collision|EventActorBeginOverlap
  (params (OtherActor :type Actor%20Object%20Reference)))

(event EventTick
  (params (DeltaSeconds :type Float%20%28single-precision%29)))

(fn ConstructionScript
  (bind _light (Variables|Default|GetLight))
  (bind _light_2 (Variables|Default|GetLight))
  (switch Utilities|FlowControl|Switch|SwitchonENUM_Light (Variables|Default|GetLightColor)
    (:NewEnumerator1
      (Rendering|Components|Light|SetLightColor _light (Variables|Default|GetPurple) true))
    (:NewEnumerator0
      (Rendering|Components|Light|SetLightColor _light (Variables|Default|GetRed) true))
    (:NewEnumerator2
      (Rendering|Components|Light|SetLightColor _light_2 (Variables|Default|GetBlue) true))
    (:NewEnumerator3
      (Rendering|Components|Light|SetLightColor _light_2 (Variables|Default|GetGreen) true))))